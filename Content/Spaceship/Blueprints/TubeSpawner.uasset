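; Spawner for the spaceship game's endless-style tube, chaining Tunnel actors and scattering pickups and hazards.
; On BeginPlay it clears existing tunnels, then builds a starting run from the player pawn, attaching each at the previous SpawnPoint.
; Each tunnel stores a spawner reference; chained spawns scatter random mines, coins and speed modifiers from the new tunnel's SpawnPoint.
; RandomChecker rerolls at every comparison, so its thresholds are not true weights.
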(event EventBeginPlay
  (CallFunction|SpawnInitialTunnels))

(event Collision|EventActorBeginOverlap
  (params (OtherActor :type Actor%20Object%20Reference)))

(event EventTick
  (params (DeltaSeconds :type Float%20%28single-precision%29)))

(fn ConstructionScript)

(fn SpawnTunnel
  (params (SpawnLocation :type Vector))
  (bind _returnvalue (Game|SpawnActorfromClass "/Game/Spaceship/Blueprints/Tunnel.Tunnel_C" (Math|Transform|MakeTransform SpawnLocation "0, 0, 0" "1,1,1") "Undefined" 0 0))
  (bind _output_get (Variables|Default|SetNewestTunnel _returnvalue))
  (Variables|/Game/Spaceship/Blueprints/Tunnel.Tunnel_C|SetTunnelSpawner _output_get self))

(fn SpawnTunnelatSpawnPoint
  (bind _newesttunnel (Variables|Default|GetNewestTunnel))
  (bind _spawnpoint (Variables|/Game/Spaceship/Blueprints/Tunnel.Tunnel_C|GetSpawnPoint _newesttunnel))
  (bind _returnvalue (Transformation|GetWorldLocation _spawnpoint))
  (CallFunction|SpawnTunnel _returnvalue)
  (CallFunction|SpawnRandomDeBuf _returnvalue))

(fn SpawnInitialTunnels
  (Utilities|FlowControl|Sequence
    (:then_0
      (bind _outactors (Actor|GetAllActorsOfClass "/Game/Spaceship/Blueprints/Tunnel.Tunnel_C"))
      (for _array_element _outactors
        (Actor|DestroyActor _array_element)))
    (:then_1
      (for _index (range 0 2)
        (Utilities|IsValid (Variables|Default|GetNewestTunnel)
          (:Is%20Valid
            (CallFunction|SpawnTunnelatSpawnPoint))
          (:Is%20Not%20Valid
            (CallFunction|SpawnTunnel (Transformation|GetActorLocation (Game|Player|GetPlayerPawn 0)))))))))

(fn SpawnRandomDeBuf
  (params (Location :type Vector))
  (for _index (range 0 5)
    (bind (_actor _create _scale) (CallFunction|RandomChecker))
    (if _create
      (Game|SpawnActorfromClass _actor (Math|Transform|MakeTransform (+ Location (Math|Vector|MakeVector (* _index (Math|Random|RandomFloatinRange 2e+02 4e+02)) (Math|Random|RandomFloatinRange -3e+02 3e+02) (Math|Random|RandomFloatinRange -3e+02 3e+02))) "0, 0, 0" _scale) "Undefined" 0 0))))

(fn RandomChecker
  (bind _returnvalue (Math|Random|RandomFloat))
  (bind _returnvalue_2 (Math|Random|RandomFloat))
  (bind _returnvalue_3 (Math|Random|RandomFloat))
  (bind _returnvalue_4 (Math|Random|RandomFloat))
  (if (and (< _returnvalue_2 0.45) (>= _returnvalue_2 0.0))
    (return "/Game/Spaceship/Blueprints/Mine.Mine_C" true "1.100000,1.100000,1.100000")
    (elif (and (< _returnvalue_3 0.75) (>= _returnvalue_3 0.45))
      (return "/Game/Spaceship/Blueprints/Coin.Coin_C" true "6.000000,6.000000,6.000000")
      (elif (and (< _returnvalue_4 0.8) (>= _returnvalue_4 0.75))
        (return "/Game/Spaceship/Blueprints/HighSpeed.HighSpeed_C" true "2.000000,2.000000,2.000000")
        (elif (and (<= _returnvalue 0.9) (>= _returnvalue 0.8))
          (return "/Game/Spaceship/Blueprints/LowSpeed.LowSpeed_C" true "2.000000,2.000000,2.000000")
          (else
            (return "/Game/Spaceship/Blueprints/LowSpeed.LowSpeed_C" false "0.000000, 0, 0")))))))